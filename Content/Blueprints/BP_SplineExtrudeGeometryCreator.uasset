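; BP_SplineExtrudeGeometryCreator creates extruded geometry along a spline at runtime and keeps it in step with edits to its control points.
; BeginPlay passes the control point file path, texture path and width to setup, creates the geometry, then copies ControlPoints into UpdatedControlPoints.
; Tick polls that copy against ControlPoints by count, then element by element, calling UpdateControlPoints once on any difference.
; The geometry functions are defined outside this Blueprint.
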(event EventTick
  (params (DeltaSeconds :type Float%20%28single-precision%29))
  (if (!= (Utilities|Array|Length (Variables|Default|GetControlPoints)) (Utilities|Array|Length (Variables|Default|GetUpdatedControlPoints)))
    (Class|SplineExtrudeGeometryCreater|UpdateControlPoints (Variables|Default|GetUpdatedControlPoints))
    (else
      (bind _index (Utilities|FlowControl|ForLoopwithBreak 0 (- (Utilities|Array|Length (Variables|Default|GetUpdatedControlPoints)) 1) :!label _label)
        (:LoopBody
          (if (Class|KismetMathLibrary|NotEqualExactlyVectorVector (Utilities|Array|Get(acopy) (Variables|Default|GetUpdatedControlPoints) _index) (Utilities|Array|Get(acopy) (Variables|Default|GetControlPoints) _index))
            (Class|SplineExtrudeGeometryCreater|UpdateControlPoints (Variables|Default|GetUpdatedControlPoints))
            (goto _label Break)))))))

(event EventBeginPlay
  (Class|SplineExtrudeGeometryCreater|SetExtrudeGeometryProperties (Variables|FilePaths|GetSpline%20Control%20Points%20File%20Path) (Variables|FilePaths|GetTexture%20File%20Path) (Variables|ExtrudeGeometry|GetWidth%20Of%20Extrude%20Geometry))
  (Class|SplineExtrudeGeometryCreater|CreateExtrudeGeometry)
  (Variables|Default|SetUpdatedControlPoints (Variables|Default|GetControlPoints)))

(fn ConstructionScript)